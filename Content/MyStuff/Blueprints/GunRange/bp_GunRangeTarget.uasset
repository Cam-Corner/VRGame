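; Gun range target actor that slides along its forward axis to a requested range, capped between zero and a maximum.
; Range setters clamp the goal distance and play a button sound through the AudioManager actor.
; BeginPlay derives the zero-range origin from its placed position.
; MoveTarget, not called within this file, eases toward the goal with a delta-time Lerp and writes the goal, divided by 100, to the supplied widget.
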(event EventBeginPlay
  (bind _currentdistance (Variables|Default|GetCurrentDistance))
  (Variables|Default|SetDirection (Math|Vector|GetForwardVector (Variables|Default|GetDefaultSceneRoot)))
  (Variables|Default|SetStartLocation (+ (Transformation|GetActorLocation) (* (* (Transformation|GetActorForwardVector) -1.0) _currentdistance)))
  (Variables|Default|SetGoToRange _currentdistance))

(fn ConstructionScript)

(fn GetRange
  (return (/ (Variables|Default|GetCurrentDistance) 1e+02)))

(fn SetMovetoRange
  (params (GoToRange :type Float%20%28single-precision%29))
  (Variables|Default|SetGoToRange GoToRange)
  (CallFunction|ClampRange)
  (CallFunction|PlayButtonPressedSound))

(fn AddtoRange
  (params (AddAmount :type Float%20%28single-precision%29))
  (Variables|Default|SetGoToRange (+ AddAmount (Variables|Default|GetGoToRange)))
  (CallFunction|ClampRange)
  (CallFunction|PlayButtonPressedSound))

(fn ClampRange
  (bind _maxmoverange (Variables|Default|GetMaxMoveRange))
  (if (> (Variables|Default|GetGoToRange) _maxmoverange)
    (Variables|Default|SetGoToRange _maxmoverange))
  (if (< (Variables|Default|GetGoToRange) 0.0)
    (Variables|Default|SetGoToRange 0.0)))

(fn MoveTarget
  (params (UWTarget :type UW%20Target%20Controller%20Object%20Reference))
  (bind _output_get (Variables|Default|SetCurrentDistance (Math|Float|Lerp (Variables|Default|GetCurrentDistance) (Variables|Default|GetGoToRange) (* (Utilities|Time|GetWorldDeltaSeconds) 4.0))))
  (Transformation|SetActorLocation (+ (* (Variables|Default|GetDirection) _output_get) (Variables|Default|GetStartLocation)) false false)
  (Default|SetText UWTarget (/ (Variables|Default|GetGoToRange) 1e+02)))

(fn PlayButtonPressedSound
  (bind _returnvalue (Actor|GetActorOfClass "/Script/VRGame.AudioManager"))
  (Class|AudioManager|PlayAudioClip _returnvalue (Variables|Default|GetButtonPressedSound) "0, 0, 0"))