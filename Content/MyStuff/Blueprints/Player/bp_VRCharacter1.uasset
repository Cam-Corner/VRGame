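; VR player character that uses floor-level tracking and owns an in-game menu actor.
; On BeginPlay it spawns the menu hidden and scaled down, passing itself as owning character.
; The menu button or ToggleMenu shows or hides it, placing it ahead of the camera facing the player and loading settings on show.
; H and G keys each add a VR character component and set its walk speed, fast or slower.
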(event Custom|ToggleMenu
  (bind _vrcamera (Variables|Default|GetVRCamera))
  (bind _ingamemenu (Variables|Default|GetInGameMenu))
  (bind _returnvalue (Transformation|GetWorldRotation _vrcamera))
  (bind _rootcomponent (Variables|/Script/Engine.Actor|GetRootComponent _ingamemenu))
  (bind (_roll _pitch _yaw) (Math|Rotator|BreakRotator _returnvalue))
  (if (Rendering|IsVisible _rootcomponent)
    (Components|Activation|SetActive _rootcomponent false false)
    (Rendering|SetVisibility _rootcomponent false false)
    (else
      (Components|Activation|SetActive _rootcomponent true false)
      (Rendering|SetVisibility _rootcomponent true false)
      (Transformation|SetWorldRotation _rootcomponent (Math|Rotator|MakeRotator 1.8e+02 (+ _pitch 1.8e+02) _yaw) false false)
      (Transformation|SetWorldLocation _rootcomponent (+ (Transformation|GetWorldLocation _vrcamera) (* (Math|Vector|GetForwardVector _vrcamera) 1e+02)) false false)
      (Default|LoadSettings (Variables|Default|GetInGameMenu)))))

(event EventBeginPlay
  (Class|HeadMountedDisplayFunctionLibrary|SetTrackingOrigin "Floor")
  (bind _returnvalue (Game|SpawnActorfromClass "/Game/MyStuff/Blueprints/Player/bp_InGameMenu.bp_InGameMenu_C" (Transformation|GetActorTransform) "Undefined" 0 0))
  (bind _output_get (Variables|Default|SetInGameMenu _returnvalue))
  (Default|SetVRCharacter _output_get self)
  (Rendering|SetVisibility (Variables|/Script/Engine.Actor|GetRootComponent _output_get) false false)
  (Components|Activation|SetActive (Variables|/Script/Engine.Actor|GetRootComponent _output_get) false false)
  (Transformation|SetWorldScale3D (Variables|/Script/Engine.Actor|GetRootComponent _output_get) "0.100000,0.100000,0.100000"))

(event Collision|EventActorBeginOverlap
  (params (OtherActor :type Actor%20Object%20Reference)))

(event EventTick
  (params (DeltaSeconds :type Float%20%28single-precision%29)))

(event Input|ActionEvents|InputActionMenuButton
  (params (Key :type Key%20Structure :default "None"))
  (bind _vrcamera (Variables|Default|GetVRCamera))
  (bind _ingamemenu (Variables|Default|GetInGameMenu))
  (bind _returnvalue (Transformation|GetWorldRotation _vrcamera))
  (bind _rootcomponent (Variables|/Script/Engine.Actor|GetRootComponent _ingamemenu))
  (bind (_roll _pitch _yaw) (Math|Rotator|BreakRotator _returnvalue))
  (:Pressed
    (if (Rendering|IsVisible _rootcomponent)
      (Components|Activation|SetActive _rootcomponent false false)
      (Rendering|SetVisibility _rootcomponent false false)
      (else
        (Components|Activation|SetActive _rootcomponent true false)
        (Rendering|SetVisibility _rootcomponent true false)
        (Transformation|SetWorldRotation _rootcomponent (Math|Rotator|MakeRotator 1.8e+02 (+ _pitch 1.8e+02) _yaw) false false)
        (Transformation|SetWorldLocation _rootcomponent (+ (Transformation|GetWorldLocation _vrcamera) (* (Math|Vector|GetForwardVector _vrcamera) 1e+02)) false false)
        (Default|LoadSettings (Variables|Default|GetInGameMenu))))))

(event Input|KeyboardEvents|H
  (params (Key :type Key%20Structure :default "None"))
  (:Pressed
    (bind _returnvalue (AddComponent|AddVRCharacterComponent))
    (Class|VRCharacterComponent|SetWalkSpeed _returnvalue 1e+03)))

(event Input|KeyboardEvents|G
  (params (Key :type Key%20Structure :default "None"))
  (:Pressed
    (bind _returnvalue (AddComponent|AddVRCharacterComponent))
    (Class|VRCharacterComponent|SetWalkSpeed _returnvalue 6e+02)))

(fn ConstructionScript)