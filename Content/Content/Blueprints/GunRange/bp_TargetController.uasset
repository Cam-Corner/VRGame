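; Gun range controller actor that links a widget component's UW_TargetController UI to a target it references.
; On BeginPlay it passes itself to the widget and shows the target's current range as text.
; Every Tick it calls MoveTarget on the target with that widget as the argument.
; GetTarget exposes the target reference to other Blueprints.
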(event EventBeginPlay
  (bind _asuw_target_controller (Utilities|Casting|CastToUW_TargetController (UserInterface|GetWidget (Variables|Default|GetWidget))))
  (Default|SetTarget _asuw_target_controller self)
  (bind _range (Default|GetRange (Variables|Default|GetTarget)))
  (Default|SetText _asuw_target_controller _range))

(event Collision|EventActorBeginOverlap
  (params (OtherActor :type Actor%20Object%20Reference)))

(event EventTick
  (params (DeltaSeconds :type Float%20%28single-precision%29))
  (bind _asuw_target_controller (Utilities|Casting|CastToUW_TargetController (UserInterface|GetWidget (Variables|Default|GetWidget))))
  (Default|MoveTarget (Variables|Default|GetTarget) _asuw_target_controller))

(fn ConstructionScript)

(fn GetTarget
  (return (Variables|Default|GetTarget)))