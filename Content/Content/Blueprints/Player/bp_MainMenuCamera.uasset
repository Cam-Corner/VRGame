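; Main menu camera Blueprint that supports both VR and flat-screen interaction with the host/join menu.
; Left and right triggers act as left mouse clicks through their own widget interaction components.
; Without an enabled headset, the UnPossess action hides BpHostJoin, adds the menu widget to the viewport and shows the cursor.
; It forces windowed 720p on BeginPlay and on that switch, and Slash quits the game.
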(event EventBeginPlay
  (Development|ExecuteConsoleCommand "r.SetRes 1280x720w" 0))

(event Input|ActionEvents|InputActionUnPossess
  (params (Key :type Key%20Structure))
  (:Pressed
    (if (not (Class|HeadMountedDisplayFunctionLibrary|IsHeadMountedDisplayEnabled))
      (Rendering|SetVisibility (Variables|Default|Getbp_HostJoin) false false)
      (bind _returnvalue (Game|ConstructObjectfromClass "/Game/Content/Blueprints/UserWidgets/bp_UW_HostJoinMenu.bp_UW_HostJoinMenu_C" self))
      (UserInterface|Viewport|AddtoViewport _returnvalue 0)
      (Development|ExecuteConsoleCommand "r.SetRes 1280x720w" 0)
      (Variables|/Script/Engine.PlayerController|SetbShowMouseCursor (Game|GetPlayerController 0) true))))

(event Input|AxisEvents|InputAxisRightTrigger
  (params (AxisValue :type Float%20%28single-precision%29))
  (if (> AxisValue 0.5)
    (Class|WidgetInteractionComponent|PressPointerKey (Variables|Default|GetRightWI) "LeftMouseButton")
    (else
      (Class|WidgetInteractionComponent|ReleasePointerKey (Variables|Default|GetRightWI) "LeftMouseButton"))))

(event Input|AxisEvents|InputAxisLeftTrigger
  (params (AxisValue :type Float%20%28single-precision%29))
  (if (> AxisValue 0.5)
    (Class|WidgetInteractionComponent|PressPointerKey (Variables|Default|GetLeftWI) "LeftMouseButton")
    (else
      (Class|WidgetInteractionComponent|ReleasePointerKey (Variables|Default|GetLeftWI) "LeftMouseButton"))))

(event Input|KeyboardEvents|Slash
  (params (Key :type Key%20Structure))
  (:Pressed
    (Game|QuitGame 0 "Quit" false)))

(fn ConstructionScript)